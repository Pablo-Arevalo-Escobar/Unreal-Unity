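; B_GridTile is a grid tile actor that shows its selection state through custom depth rendering on its TileMesh.
; On BeginPlay it binds to OnSelectedTrigger; selection enables custom depth with a fixed stencil value, suited to a stencil-based highlight, and deselection calls Deselect to disable it.
; Tick and overlap events do nothing, and a debug name label is left unconnected.
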(event Custom|OnSelectedTrigger_Event
  (params (IsSelected :type Boolean))
  (bind _tilemesh (Variables|Default|GetTileMesh))
  (if IsSelected
    (Rendering|SetRenderCustomDepth _tilemesh true)
    (Rendering|SetCustomDepthStencilValue _tilemesh 2)
    (else
      (CallFunction|EventDeselect))))

(event Custom|Event%20Deselect
  (Rendering|SetRenderCustomDepth (Variables|Default|GetTileMesh) false))

(event Collision|EventActorBeginOverlap
  (params (OtherActor :type Actor%20Object%20Reference)))

(event EventTick
  (params (DeltaSeconds :type Float%20%28single-precision%29)))

(event EventBeginPlay
  (EventDispatchers|BindEventtoOnSelectedTrigger (delegate Custom|OnSelectedTrigger_Event)))

(fn ConstructionScript)